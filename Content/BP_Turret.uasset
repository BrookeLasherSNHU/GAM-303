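; BP_Turret is a turret that tracks the player character and fires projectiles at it when in range.
; Each tick it finds the player with GetActorOfClass, turns its Arrow component toward them and counts down a cooldown.
; When the player is close enough and the cooldown has expired, it spawns a BP_TurretProjectile at its own transform, passing the Arrow's forward vector as direction and setting a limited lifespan.
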(event `self.ReceiveTick`
  (params (DeltaSeconds :type "Float (single-precision)"))
  (bind _returnvalue (`GameplayStatics.GetActorOfClass` "/Game/PlayerCharacter.PlayerCharacter_C"))
  (`SceneComponent.K2_SetWorldRotation` (`self.Arrow`) (`KismetMathLibrary.FindLookAtRotation` (`self.K2_GetActorLocation`) (`self.K2_GetActorLocation` _returnvalue)) false false)
  (bind _output_get (set `self.ProjectileCooldown` (- (`self.ProjectileCooldown`) DeltaSeconds)))
  (if (and (<= (`KismetMathLibrary.Vector_Distance` (`self.K2_GetActorLocation`) (`self.K2_GetActorLocation` _returnvalue)) 1000.0) (<= _output_get 0.0))
    (bind _returnvalue_2 (`|SpawnActorFromClass` "/Game/BP_TurretProjectile.BP_TurretProjectile_C" (`self.GetTransform`) "AlwaysSpawn" "MultiplyWithRoot" null null))
    (set `/Game/BP_TurretProjectile.Direction` (`SceneComponent.GetForwardVector` (`self.Arrow`)) _returnvalue_2)
    (`self.SetLifeSpan` _returnvalue_2 5.0)
    (set `self.ProjectileCooldown` 5.0)))

(fn `UserConstructionScript`)