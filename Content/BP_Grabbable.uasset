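; BP_Grabbable is an actor with a cube that the player can pick up and drop by interacting with it.
; Interact stores the calling player, toggles the grabbed state and switches the cube's gravity off while held.
; While grabbed, Tick moves the cube with a swept SetWorldLocation to a fixed distance in front of that player's camera.
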(event `self.ReceiveTick`
  (params (DeltaSeconds :type "Float (single-precision)"))
  (bind _lastplayer (`self.LastPlayer`))
  (if (`self.IsGrabbed`)
    (`SceneComponent.K2_SetWorldLocation` (`self.Cube`) (+ (* (`SceneComponent.GetForwardVector` (`/Game/PlayerCharacter.Camera` _lastplayer)) (100.0 100.0 100.0)) (`SceneComponent.K2_GetComponentLocation` (`/Game/PlayerCharacter.Camera` _lastplayer))) true false)))

(event `/Game/Interactable.Interact`
  (params (`Player Ref` :type "/Game/PlayerCharacter Object Reference"))
  (bind _returnvalue (not (`self.IsGrabbed`)))
  (set `self.LastPlayer` `Player Ref`)
  (set `self.IsGrabbed` _returnvalue)
  (`PrimitiveComponent.SetEnableGravity` (`self.Cube`) _returnvalue))

(fn `UserConstructionScript`)