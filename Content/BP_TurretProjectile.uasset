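; BP_TurretProjectile is a projectile actor, named for turret fire, that moves itself on Tick without a movement component.
; Each tick subtracts delta time from Lifespan, then branches on whether it has reached zero.
; The branch reads inverted: at or below zero it teleports along Direction by a fixed, frame-rate-dependent step without sweeping, while a positive Lifespan destroys the actor.
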(event `self.ReceiveTick`
  (params (DeltaSeconds :type "Float (single-precision)"))
  (bind _output_get (set `self.Lifespan` (- (`self.Lifespan`) DeltaSeconds)))
  (if (<= _output_get 0.0)
    (`self.K2_SetActorLocation` (+ (`self.K2_GetActorLocation`) (* (`self.Direction`) (6.0 6.0 6.0))) false true)
    (else
      (`self.K2_DestroyActor`))))

(fn `UserConstructionScript`)