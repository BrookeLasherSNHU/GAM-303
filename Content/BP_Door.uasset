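; BP_Door is an interactable door that swings open and closed on alternate Interact calls.
; A FlipFlop plays or reverses a Timeline that lerps the Arrow component's relative yaw up to a quarter turn.
; The swing side comes from a dot product of the door's forward vector and the player's direction to world origin, not to the door, re-evaluated on each update.
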(event `/Game/Interactable.Interact`
  (params (`Player Ref` :type "/Game/PlayerCharacter Object Reference"))
  (`/Engine/EditorBlueprintResources/StandardMacros.FlipFlop`
    (:`A`
      (bind (_direction _alpha) (`Timeline|Timeline` :!label _label)
        (:`Update`
          (`SceneComponent.K2_SetRelativeRotation` (`self.Arrow`) (`KismetMathLibrary.MakeRotator` 0.0 0.0 (`KismetMathLibrary.Lerp` 0.0 (select `bool` (< (`KismetMathLibrary.Dot_VectorVector` (`KismetMathLibrary.GetDirectionUnitVector` (`self.K2_GetActorLocation` `Player Ref`)) (`self.GetActorForwardVector`)) 0.0) :`false` -90.0 :`true` 90.0 :!type "Float (single-precision)") _alpha)) false false))))
    (:`B`
      (goto _label :!via `Reverse`))))

(fn `UserConstructionScript`)